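; Master Blueprint for holdable items, providing item setup and chained melee light attacks for child items.
; Construction looks up ItemID in DT_ItemList to fill ItemDetails and set the mesh.
; LightAttack steps a three-hit combo counter on the character's component, flags the array's final attack, and plays montages through the character's server event.
; Empty ChainLightAttack and ChainHeavyAttack hooks let children mix combos; only the light hook is called here.
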(event `self.ReceiveBeginPlay`
  ;[0.1719 0.1719 0.1719] Sets a reference to the character
  (bind _asbp_master_character (cast `/Game/Wizard_World/Blueprints/Character/BP_MasterCharacter` (`GameplayStatics.GetPlayerCharacter` 0)))
  (set `self.CharacterRef` _asbp_master_character))

(event `ChainLightAttack`
  (params (ChainLightAttack :type Integer))
  ;[0.1719 0.1719 0.1719] Chain Attacks ( used in children Blueprints o Mix and Match light/heavy chain attacks
)

(event `ChainHeavyAttack`
  (params (ChainHeavyAttack :type Integer))
  ;[0.1719 0.1719 0.1719] Chain Attacks ( used in children Blueprints o Mix and Match light/heavy chain attacks
)

(event `LightAttack`
  (bind _characterref (`self.CharacterRef`))
  (bind _characterref_2 (`self.CharacterRef`))
  (bind _characterref_3 (`self.CharacterRef`))
  (bind _output (`|GetArrayItem` (`.MeleeLightAttacks_8_A107C590497C3D2B169337BE43EAB33D` (break `/Game/Wizard_World/Blueprints/Data/Structures/ST_AnimationDetails` (`.AnimationDetails_32_7E2BF6E1430680CCC710CB9E068A8700` (break `/Game/Wizard_World/Blueprints/Data/Structures/ST_ItemDetails` (`self.ItemDetails`))))) (`/Game/Wizard_World/Blueprints/Components/BPC_CharacterComponent.ChainLightAttack` (`/Game/Wizard_World/Blueprints/Character/BP_MasterCharacter.BPC_CharacterComponent` (`self.CharacterRef`)))))
  ;[0.1719 0.1719 0.1719] Light Attack
  ;;[0.1719 0.1719 0.1719] Check if the last number in the weapon detail light attack array is = to the chain attack +1 (Final Attack is next if true)
  (if (== (`KismetArrayLibrary.Array_Length` (`.MeleeLightAttacks_8_A107C590497C3D2B169337BE43EAB33D` (break `/Game/Wizard_World/Blueprints/Data/Structures/ST_AnimationDetails` (`.AnimationDetails_32_7E2BF6E1430680CCC710CB9E068A8700` (break `/Game/Wizard_World/Blueprints/Data/Structures/ST_ItemDetails` (`self.ItemDetails`)))))) (+ (`/Game/Wizard_World/Blueprints/Components/BPC_CharacterComponent.ChainLightAttack` (`/Game/Wizard_World/Blueprints/Character/BP_MasterCharacter.BPC_CharacterComponent` (`self.CharacterRef`))) 1))
    ;;[0.1719 0.1719 0.1719] Set final attack in a combo
    (set `/Game/Wizard_World/Blueprints/Components/BPC_CharacterComponent.bLastAttack` true (`/Game/Wizard_World/Blueprints/Character/BP_MasterCharacter.BPC_CharacterComponent` (`self.CharacterRef`))))
  ;;[0.1719 0.1719 0.1719] Switch between each attack (each time you attack, +1 is added unless it is the final attack, then we will reset it to 0)
  (switch `int` (`/Game/Wizard_World/Blueprints/Components/BPC_CharacterComponent.ChainLightAttack` (`/Game/Wizard_World/Blueprints/Character/BP_MasterCharacter.BPC_CharacterComponent` (`self.CharacterRef`)))
    (:`0`
      ;;[0.1719 0.1719 0.1719] Play attack animation montage depending on the current chain light attack ID
      (`/Game/Wizard_World/Blueprints/Character/BP_MasterCharacter.SERVER_PlayMontage` _characterref (`Character.Mesh` _characterref) _output 1.0 0.0 "None")
      ;;[0.1719 0.1719 0.1719] Set the current chain attack ref to the chain light attack event ref (to be used by children BP's to Mix/Match Chain attacks)
      (`self.ChainLightAttack` (`/Game/Wizard_World/Blueprints/Components/BPC_CharacterComponent.ChainLightAttack` (`/Game/Wizard_World/Blueprints/Character/BP_MasterCharacter.BPC_CharacterComponent` (`self.CharacterRef`))))
      (set `/Game/Wizard_World/Blueprints/Components/BPC_CharacterComponent.ChainLightAttack` 1 (`/Game/Wizard_World/Blueprints/Character/BP_MasterCharacter.BPC_CharacterComponent` (`self.CharacterRef`))))
    (:`1`
      (`/Game/Wizard_World/Blueprints/Character/BP_MasterCharacter.SERVER_PlayMontage` _characterref_2 (`Character.Mesh` _characterref_2) _output 1.0 0.0 "None")
      (`self.ChainLightAttack` (`/Game/Wizard_World/Blueprints/Components/BPC_CharacterComponent.ChainLightAttack` (`/Game/Wizard_World/Blueprints/Character/BP_MasterCharacter.BPC_CharacterComponent` (`self.CharacterRef`))))
      (set `/Game/Wizard_World/Blueprints/Components/BPC_CharacterComponent.ChainLightAttack` 2 (`/Game/Wizard_World/Blueprints/Character/BP_MasterCharacter.BPC_CharacterComponent` (`self.CharacterRef`))))
    (:`2`
      (`/Game/Wizard_World/Blueprints/Character/BP_MasterCharacter.SERVER_PlayMontage` _characterref_3 (`Character.Mesh` _characterref_3) _output 1.0 0.0 "None")
      (`self.ChainLightAttack` (`/Game/Wizard_World/Blueprints/Components/BPC_CharacterComponent.ChainLightAttack` (`/Game/Wizard_World/Blueprints/Character/BP_MasterCharacter.BPC_CharacterComponent` (`self.CharacterRef`))))
      (set `/Game/Wizard_World/Blueprints/Components/BPC_CharacterComponent.ChainLightAttack` 0 (`/Game/Wizard_World/Blueprints/Character/BP_MasterCharacter.BPC_CharacterComponent` (`self.CharacterRef`))))))

(fn `UserConstructionScript`
  ;[0.1719 0.1719 0.1719] Set data determined by the info written in the DT_ItemList. ItemID in each itemBP will determine the row used for the items details
  (bind _returnvalue (`|GetDataTableRow` "/Game/Wizard_World/Blueprints/Data/DataTables/DT_ItemList.DT_ItemList" (`self.ItemID`))
    (:`then`
      (set `self.ItemDetails` _returnvalue)
      (`StaticMeshComponent.SetStaticMesh` (`self.HoldableMesh`) (`.ItemMesh_9_B60A0C0547D20087E6F10FA07584197C` (break `/Game/Wizard_World/Blueprints/Data/Structures/ST_ItemDetails` (`self.ItemDetails`)))))))